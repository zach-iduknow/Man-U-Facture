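; BP_HarvestTool is a harvest tool assembled from two parts, ToolHead and ToolBase, which supply its meshes.
; On BeginPlay, a validity macro checks both parts and, only when both are valid, calls SetToolMesh.
; SetToolMesh applies the ToolHead mesh to HandleMesh and the ToolBase mesh to HeadMesh, so the head part's mesh lands on the handle component.
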(event EventBeginPlay
  (Utilities|AreToolPartsValid?
    (:Valid
      (CallFunction|SetToolMesh))))

(event Collision|EventActorBeginOverlap
  (params (OtherActor :type Actor%20Object%20Reference)))

(event EventTick
  (params (DeltaSeconds :type Float%20%28single-precision%29)))

(fn ConstructionScript)

(fn SetToolMesh
  (Components|StaticMesh|SetStaticMesh (Variables|Default|GetHandleMesh) (Class|ToolComponent|GetMesh (Variables|ToolParts|GetToolHead)))
  (Components|StaticMesh|SetStaticMesh (Variables|Default|GetHeadMesh) (Class|ToolComponent|GetMesh (Variables|ToolParts|GetToolBase))))